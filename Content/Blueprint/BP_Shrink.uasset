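; BP_Shrink is a fireable ability that toggles its owning actor between original size and one-third scale.
; Fire adds a Niagara effect to the owner and picks the target by comparing the owner's scale with OriginalSize, which construction records from the Blueprint's own scale.
; SizeChange runs a timeline that lerps the owner's scale to the target, resetting and activating the effect on every update.
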(event `SizeChange`
  (bind (_direction _newtrack_0) (`Timeline|Timeline` :!via `PlayFromStart`)
    (:`Update`
      (`self.SetActorScale3D` (`self.Player`) (`KismetMathLibrary.VLerp` (`self.Current Scale`) (`self.New Size`) _newtrack_0))
      (`ActorComponent.SetActive` (`self.Shrink Fx`) true true))))

(fn `Fire`
  (returns (ReturnValue :type Boolean))
  (bind _original_size (`self.Original Size`))
  (bind _player (`self.Player`))
  (bind _output_get (set `self.Player` (`self.GetOwner`)))
  (bind _returnvalue (`AddComponent|NODE_AddNiagaraComponent-2` :`self` _output_get))
  (`AddComponent|NODE_AddNiagaraComponent-3` :`self` _player)
  (set `self.Shrink Fx` _returnvalue)
  (if (== (`self.GetActorScale3D` _player) (`self.Original Size`))
    (set `self.New Size` (/ _original_size (`KismetMathLibrary.Conv_DoubleToVector` 3.0)))
    (else
      (set `self.New Size` _original_size)))
  (set `self.Current Scale` (`self.GetActorScale3D` (`self.Player`)))
  (`self.SizeChange`)
  (return true))

(fn `UserConstructionScript`
  (set `self.Original Size` (`self.GetActorScale3D`)))