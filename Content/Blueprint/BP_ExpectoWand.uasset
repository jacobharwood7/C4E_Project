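; Wand that casts an Expecto Patronum shield spell which stays attached to its muzzle.
; Fire destroys any existing shield, spawns a new BP_ExpectoPatronum and calls Update, which unpauses a looping timer created paused at BeginPlay.
; At roughly 60 Hz, Update moves the shield to the muzzle and feeds muzzle position and a forward point into its Niagara parameters.
; EndPlay destroys the shield.
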(event `self.ReceiveBeginPlay`
  (bind _returnvalue (`KismetSystemLibrary.K2_SetTimer` null "Update" 0.016 true))
  (bind _output_get (set `self.Shield Timer` _returnvalue))
  (`KismetSystemLibrary.K2_PauseTimerHandle` _output_get))

(event `self.ReceiveEndPlay`
  (params (EndPlayReason :type "EEndPlayReason Enum" :default "Destroyed"))
  (`self.K2_DestroyActor` (`self.ShieldSpell`)))

(fn `Fire`
  (returns (ReturnValue :type Boolean))
  (bind _shieldspell (`self.ShieldSpell`)
    (:`then`
      (`self.K2_DestroyActor` _shieldspell))
    (:`else`
      _))
  (bind _returnvalue (`|SpawnActorFromClass` "/Game/VFX/Spells/BP_ExpectoPatronum.BP_ExpectoPatronum_C" (`KismetMathLibrary.Conv_VectorToTransform` (`SceneComponent.K2_GetComponentLocation` (`self._Muzzle`))) "Undefined" "MultiplyWithRoot" null null))
  (set `self.ShieldSpell` _returnvalue)
  (`self.Update`)
  (return true))

(fn `Update`
  (bind __muzzle (`self._Muzzle`))
  (bind _shieldspell (`self.ShieldSpell`))
  (bind _returnvalue (`SceneComponent.K2_GetComponentLocation` __muzzle))
  (bind _niagara (`/Game/VFX/Spells/BP_ExpectoPatronum.Niagara` _shieldspell))
  (`KismetSystemLibrary.K2_UnPauseTimerHandle` (`self.Shield Timer`))
  (`self.K2_SetActorLocation` _shieldspell _returnvalue false false)
  (`FXSystemComponent.SetVectorParameter` _niagara "User.ForwardV" (+ _returnvalue (`SceneComponent.GetForwardVector` __muzzle)))
  (`FXSystemComponent.SetVectorParameter` _niagara "User.Point" (`SceneComponent.K2_GetComponentLocation` __muzzle)))

(fn `UserConstructionScript`)