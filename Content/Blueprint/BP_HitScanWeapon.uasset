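; BP_HitScanWeapon is a hitscan weapon that fires a green Niagara zap beam and damages what it hits.
; Fire replaces the previous beam, line-traces forward from the Muzzle on Visibility with debug drawing, applies damage on a hit and returns whether it hit.
; The beam ends at the impact or trace end, while a looping timer, paused until firing, runs Update to keep its start on the moving Muzzle.
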(event `self.ReceiveBeginPlay`
  (bind _returnvalue (`KismetSystemLibrary.K2_SetTimer` null "Update" 0.016 true))
  (bind _output_get (set `self.Timer for Spell` _returnvalue))
  (`KismetSystemLibrary.K2_PauseTimerHandle` _output_get))

(fn `Fire`
  (returns (ReturnValue :type Boolean))
  (bind __muzzle (`self._Muzzle`))
  (if (!= (`self.ZAP`) null)
    (`ActorComponent.K2_DestroyComponent` (`self.ZAP`)))
  (bind (_outhit _returnvalue) (`KismetSystemLibrary.LineTraceSingle` :`Start` (`SceneComponent.K2_GetComponentLocation` __muzzle) :`End` (+ (`SceneComponent.K2_GetComponentLocation` __muzzle) (* (`SceneComponent.GetForwardVector` __muzzle) 2000.0)) :`TraceChannel` "TraceTypeQuery1" :`DrawDebugType` "ForDuration"))
  (bind _returnvalue_2 (`NiagaraFunctionLibrary.SpawnSystemAtLocation` "/Game/VFX/Spells/NS_Zap_Spells.NS_Zap_Spells"))
  (set `self.ZAP` _returnvalue_2)
  (`FXSystemComponent.SetColorParameter` (`self.ZAP`) "User.Spell" (struct :`G` 1.0 :`A` 1.0))
  (`KismetSystemLibrary.K2_UnPauseTimerHandle` (`self.Timer for Spell`))
  (`FXSystemComponent.SetVectorParameter` (`self.ZAP`) "User.BeamStart" (`SceneComponent.K2_GetComponentLocation` (`self._Muzzle`)))
  (if _returnvalue
    (`GameplayStatics.ApplyDamage` (`.HitActor` (`GameplayStatics.BreakHitResult` _outhit)) (`self.Base Damage`) (`self.GetInstigatorController`) self "/Script/Engine.DamageType")
    (`FXSystemComponent.SetVectorParameter` (`self.ZAP`) "User.BeamEnd" (`.Location` (`GameplayStatics.BreakHitResult` _outhit)))
    (else
      (`FXSystemComponent.SetVectorParameter` (`self.ZAP`) "User.BeamEnd" (`.TraceEnd` (`GameplayStatics.BreakHitResult` _outhit)))))
  (`self.Update`)
  (return _returnvalue))

(fn `Update`
  (`FXSystemComponent.SetVectorParameter` (`self.ZAP`) "User.BeamStart" (`SceneComponent.K2_GetComponentLocation` (`self._Muzzle`))))

(fn `UserConstructionScript`)